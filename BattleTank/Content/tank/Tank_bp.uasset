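; Player-controllable tank Blueprint that handles camera aiming, track-driven movement and firing.
; BeginPlay passes the barrel and turret (named "Tarrel") components to their reference setters.
; Aim axes rotate an azimuth gimbal for yaw and the spring arm for pitch, scaled without delta time.
; Throttle axes drive each track directly, Forward goes through TankMovementComponent, the fire action calls Firing, and BackWard is unwired.
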(event `self.ReceiveBeginPlay`
  (`self.SetBarrelReference` (`self.TankBarrel`))
  (`self.SetTarrelReference` (`self.TankTarrel`)))

(event `InputAxis|AimAzimuth`
  (params (AxisValue :type "Float (single-precision)"))
  ;[1 1 1] Aim Input Binding
  (`SceneComponent.K2_AddLocalRotation` (`self.AzimuthGimbal`) (`KismetMathLibrary.MakeRotator` 0.0 0.0 (* AxisValue 2.0)) false false))

(event `InputAxis|LeftTraceTrottle`
  (params (AxisValue :type "Float (single-precision)"))
  ;[1 1 1] Movement Input Binding
  (`TankTrack.SetThrottle` (`self.TankTrackLeft`) AxisValue))

(event `InputAxis|RightTraceTrottle`
  (params (AxisValue :type "Float (single-precision)"))
  ;[1 1 1] Movement Input Binding
  (`TankTrack.SetThrottle` (`self.TankTrackRight`) AxisValue))

(event `InputAxis|AimElevation`
  (params (AxisValue :type "Float (single-precision)"))
  ;[1 1 1] Aim Input Binding
  (`SceneComponent.K2_AddLocalRotation` (`self.SpringArm`) (`KismetMathLibrary.MakeRotator` 0.0 (* AxisValue 2.0)) false false))

(event `InputAxis|Forward`
  (params (AxisValue :type "Float (single-precision)"))
  ;[1 1 1] Movement Input Binding
  (`TankMovementComponent.IntendMoveForward` (`self.TankMovementComponent`) AxisValue))

(event `InputAction|Firing`
  (params (Key :type "Key Structure"))
  ;[1 1 1] Aim Input Binding
  (:`Pressed`
    (`self.Firing`)))

(event `InputAxis|BackWard`
  (params (AxisValue :type "Float (single-precision)"))
  ;[1 1 1] Movement Input Binding
)

(fn `UserConstructionScript`)